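; Lobby room wall Blueprint that fires a switcher when a wall trap is pressed.
; Tick polls WallTrapState1 and calls ActivateSwitcher on Switcher once it reads Pressed, with an Executed flag limiting this to a single activation.
; An unconnected condition requiring both WallTrapState1 and WallTrapState to be pressed remains in the graph, so only the first trap matters.
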(event `self.ReceiveTick`
  (params (DeltaSeconds :type "Float (single-precision)"))
  (if (`self.Executed`)
    _
    (elif (`|EnumEquality` (`WallTrapState._State` (`self.WallTrapState1`)) "Pressed")
      (`SwitcherComponent.ActivateSwitcher` (`self.Switcher`))
      (set `self.Executed` true))))

(fn `UserConstructionScript`)