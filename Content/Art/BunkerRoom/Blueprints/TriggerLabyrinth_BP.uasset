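; One-shot trigger actor for the bunker labyrinth that shuts and locks a referenced grid door when the player walks into it.
; On overlap with PlayerCharacter, it reads the DisplaceState component on GridDoor and calls SwitchState if it is at its final position or moving.
; It then sets the component's Block flag and destroys itself, doing nothing if the door or component is missing.
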(event `DestroyTrigger`
  (`self.K2_DestroyActor`))

(event `self.ReceiveActorBeginOverlap`
  (params (OtherActor :type "Actor Object Reference"))
  (bind _griddoor (`self.GridDoor`))
  (bind _returnvalue (`self.GetComponentByClass` _griddoor "/Script/ListenToMyVoice.DisplaceState"))
  (bind __state (`DisplaceState._State` _returnvalue))
  (cast `PlayerCharacter` OtherActor)
  (`/Engine/EditorBlueprintResources/StandardMacros.IsValid` _griddoor
    (:`Is Valid`
      (`/Engine/EditorBlueprintResources/StandardMacros.IsValid` _returnvalue
        (:`Is Valid`
          (if (or (`|EnumEquality` __state "FinalPosition") (`|EnumEquality` __state "Moving"))
            (`DisplaceState.SwitchState` _returnvalue))
          (set `DisplaceState._Block` true _returnvalue)
          (`self.DestroyTrigger`))))))

(fn `UserConstructionScript`)