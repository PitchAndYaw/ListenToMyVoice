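; Diary page actor for the bunker room that stays hidden until the text on its linked Panel becomes visible.
; Each Tick until activation, it checks the Panel's TextRenderComponent and keeps itself hidden while that text is invisible.
; Once the text shows, it unhides itself, plays its FMOD audio and latches Active, so the reveal happens only once.
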(event `self.ReceiveTick`
  (params (DeltaSeconds :type "Float (single-precision)"))
  (if (`self.Active`)
    _
    (elif (`SceneComponent.IsVisible` (`self.GetComponentByClass` (`self.Panel`) "/Script/Engine.TextRenderComponent"))
      (`self.SetActorHiddenInGame` false)
      (`FMODAudioComponent.Play` (`self.FMODAudio`))
      (set `self.Active` true)
      (else
        (`self.SetActorHiddenInGame` true)))))

(fn `UserConstructionScript`)