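; CheckIfDamaged is an enemy AI behavior tree node that reports when the enemy has taken damage.
; Each tick it reads the Damaged flag from the controlled EnemyCharacter and copies it to the Damaged blackboard key.
; When the flag is set, it clears it on the character and sets the TargetPawn key to the player character, whatever the damage source.
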(event `self.ReceiveTick`
  (params (OwnerActor :type "Actor Object Reference") (DeltaSeconds :type "Float (single-precision)"))
  (bind _asenemy_controller (cast `EnemyController` OwnerActor))
  (bind _returnvalue (`AIBlueprintHelperLibrary.GetAIController` _asenemy_controller))
  (bind _asenemy_character (cast `EnemyCharacter` (`Controller.K2_GetPawn` _asenemy_controller)))
  (`/Engine/EditorBlueprintResources/StandardMacros.IsValid` _returnvalue
    (:`Is Valid`
      (if true
        (bind _returnvalue_2 (`EnemyCharacter.GetDamaged` _asenemy_character))
        (if _returnvalue_2
          (`BTFunctionLibrary.SetBlackboardValueAsBool` (`self.Damaged?`) _returnvalue_2)
          (`EnemyCharacter.SetDamaged` _asenemy_character false)
          (`BTFunctionLibrary.SetBlackboardValueAsObject` (`self.TargetPawn`) (`GameplayStatics.GetPlayerCharacter` 0))
          (else
            (`BTFunctionLibrary.SetBlackboardValueAsBool` (`self.Damaged?`) _returnvalue_2)))))))