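; Behavior tree task that picks the next waypoint for an EnemyCharacter on a linked waypoint route.
; When the enemy's location matches CurrentWaypoint almost exactly, it stores that waypoint's NextWaypoint in NewWaypoint, otherwise it clears NewWaypoint.
; Both branches finish successfully, but a failed cast returns without finishing the task.
; A helper function returns a waypoint's location, though the execute event does not call it.
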(event `self.ReceiveExecute`
  (params (OwnerActor :type "Actor Object Reference"))
  (bind _asenemy_character (cast `EnemyCharacter` OwnerActor))
  (if (== (`Actor.K2_GetActorLocation` _asenemy_character) (`Actor.K2_GetActorLocation` (`self.Current Waypoint`)))
    (bind _aswaypoint (cast `/Game/BluePrints/AI/Waypoint` (`/Game/BluePrints/AI/Waypoint.NextWaypoint` (`self.Current Waypoint`))))
    (set `self.New Waypoint` _aswaypoint)
    (else
      (set `self.New Waypoint` null)))
  (`self.FinishExecute` true))

(fn `Get Waypoint Location`
  (params (NewParam :type "/Game/BluePrints/AI/Waypoint Object Reference"))
  (returns (ReturnValue :type "Vector Structure"))
  (return (`Actor.K2_GetActorLocation` (`|ConvertAsset` NewParam))))